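; BP_HPController is a health component that tracks an actor's health and death.
; It fills health to the maximum on BeginPlay, and ReceiveDamage subtracts damage only while health remains, clamping it at zero.
; Each applied hit raises an HP-changed event with current and maximum health, preceded by a death event when health runs out.
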(event `self.ReceiveBeginPlay`
  ;[0.1182 0.15 0.0679 0.5] 시작할 때 최대체력으로
  (set `self.HealthPower` (`self.MaxHealthPower`)))

(event `ReceiveDamage`
  (params (Damage :type "Float (double-precision)"))
  ;[0.15 0.05316 0.02958 0.5] 대미지 처리 - 과정에서 죽음 및 체력 변경 이벤트도 발행
  (if (> (`self.HealthPower`) 0.0)
    (bind _output_get (set `self.HealthPower` (- (`self.HealthPower`) Damage)))
    (if (<= _output_get 0.0)
      (set `self.HealthPower` 0.0)
      (`self.OnDeadEvent`)
      (`self.OnHpChanged` (`self.HealthPower`) (`self.MaxHealthPower`))
      (else
        (`self.OnHpChanged` (`self.HealthPower`) (`self.MaxHealthPower`))))))