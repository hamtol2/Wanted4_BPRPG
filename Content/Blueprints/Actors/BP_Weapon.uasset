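; BP_Weapon is a weapon actor that characters pick up by touch and that carries a collision volume for attack checks.
; When a BP_Character overlaps the pickup sphere, the weapon passes itself to that character's OnWeaponCollected and turns the sphere's collision off.
; AttackCollision is off from BeginPlay, and the OnAttackCheckBegin and OnAttackCheckEnd events switch it between query-only and no collision.
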(event `self.ReceiveBeginPlay`
  ; 공격 콜리전 끄기
  (`PrimitiveComponent.SetCollisionEnabled` (`self.AttackCollision`) "NoCollision"))

(event `self.Sphere.OnComponentBeginOverlap`
  (params (OverlappedComponent :type "PrimitiveComponent Object Reference") (OtherActor :type "Actor Object Reference") (OtherComp :type "PrimitiveComponent Object Reference") (OtherBodyIndex :type Integer) (bFromSweep :type Boolean) (SweepResult :type "HitResult Structure (by ref)"))
  ;[0.15 0.1222 0.02238 0.5] 무기 습득 처리
  (bind _asbp_character (cast `/Game/Blueprints/Character/BP_Character` OtherActor))
  (`/Game/Blueprints/Character/BP_Character.OnWeaponCollected` _asbp_character self)
  (`PrimitiveComponent.SetCollisionEnabled` (`self.Sphere`) "NoCollision"))

(event `OnAttackCheckBegin`
  ;[0.04265 0.08571 0.15 0.5] 공격 판정 시작
  (`PrimitiveComponent.SetCollisionEnabled` (`self.AttackCollision`) "QueryOnly"))

(event `OnAttackCheckEnd`
  ;[0.15 0.02962 0.03873 0.5] 공격 판정 종료
  (`PrimitiveComponent.SetCollisionEnabled` (`self.AttackCollision`) "NoCollision"))

(fn `UserConstructionScript`)